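; Behavior tree task that sends an EnemyChracter_BP AI toward the first player's pawn.
; On AI tick, it sets the enemy's max walk speed from the WalkSpeed blackboard value, with debug prints for failed checks.
; It issues AIMoveTo to the player's current location using SmellRange as acceptance radius.
; The immediate output sets Walkto true and finishes the task successfully without waiting for arrival.
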(event EventReceiveTickAI
  (params (OwnerController :type AI%20Controller%20Object%20Reference) (ControlledPawn :type Pawn%20Object%20Reference) (DeltaSeconds :type Float%20%28single-precision%29))
  (bind _asenemy_chracter_bp (Utilities|Casting|CastToEnemyChracter_BP ControlledPawn)
    (:then
      _)
    (:CastFailed
      (Development|PrintString "gg")))
  (Utilities|IsValid (Actor|GetComponentbyClass _asenemy_chracter_bp "/Script/Engine.CharacterMovementComponent")
    (:Is%20Valid
      (Variables|/Script/Engine.CharacterMovementComponent|SetMaxWalkSpeed (Actor|GetComponentbyClass _asenemy_chracter_bp "/Script/Engine.CharacterMovementComponent") (Class|BTFunctionLibrary|GetBlackboardValueasFloat (Variables|Default|GetWalk%20Speed))))
    (:Is%20Not%20Valid
      (Development|PrintString "Hello")))
  (AI|AIMoveTo OwnerController (Transformation|GetActorLocation (Pawn|GetControlledPawn (Game|GetPlayerController 0))) 0 (Class|BTFunctionLibrary|GetBlackboardValueasFloat (Variables|Default|GetSmellRange)) "Default" "Default" true true
    (:then
      (Class|BTFunctionLibrary|SetBlackboardValueasBool (Variables|Default|GetWalkto) true)
      (AI|BehaviorTree|FinishExecute true))))