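; Enemy character that feeds a behavior-tree Blackboard and deals melee fist damage to the player.
; BeginPlay seeds patrol, range, speed and cooldown keys, spawns a socket-attached weakspot actor, then applies its health and drop rates after a short delay.
; Tick updates player distance, weakspot-hit and death keys, disabling collision once the weakspot is dead.
; Toggleable fist overlaps damage the player with camera shake and timed damage feedback.
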(event OnComponentBeginOverlap(RightFist)
  (params (OverlappedComponent :type Primitive%20Component%20Object%20Reference) (OtherActor :type Actor%20Object%20Reference) (OtherComp :type Primitive%20Component%20Object%20Reference) (OtherBodyIndex :type Integer) (bFromSweep :type Boolean) (SweepResult :type Hit%20Result%20Structure%20%28by%20ref%29))
  (bind _returnvalue (Game|GetPlayerCharacter 0))
  ;[1 1 1] Fist Hit Player (OverlapEvent)
  (if (== OtherActor _returnvalue)
    (Development|PrintString "Right hit")
    (bind _ascharater_bp (Utilities|Casting|CastToCharater_BP _returnvalue))
    (Variables|/Game/Blueprint/Charater_BP.Charater_BP_C|SetPlayerHealth _ascharater_bp (- (Variables|/Game/Blueprint/Charater_BP.Charater_BP_C|GetPlayerHealth _ascharater_bp) (Variables|PublicVariable|GetDamage%20per%20hit)))
    (Camera|PlayWorldCameraShake "/Game/Blueprint/HitShake_BP.HitShake_BP_C" (Transformation|GetActorLocation) 0.0 (Variables|Default|GetShakeValue))
    (Default|CallUpdateDamage _ascharater_bp true)
    (Utilities|FlowControl|Delay 0.967)
    (Default|CallUpdateDamage _ascharater_bp false)))

(event OnComponentBeginOverlap(LeftFist)
  (params (OverlappedComponent :type Primitive%20Component%20Object%20Reference) (OtherActor :type Actor%20Object%20Reference) (OtherComp :type Primitive%20Component%20Object%20Reference) (OtherBodyIndex :type Integer) (bFromSweep :type Boolean) (SweepResult :type Hit%20Result%20Structure%20%28by%20ref%29))
  (bind _returnvalue (Game|GetPlayerCharacter 0))
  ;[1 1 1] Fist Hit Player (OverlapEvent)
  (if (== _returnvalue OtherActor)
    (Development|PrintString "Left hit")
    (bind _ascharater_bp (Utilities|Casting|CastToCharater_BP _returnvalue))
    (Variables|/Game/Blueprint/Charater_BP.Charater_BP_C|SetPlayerHealth _ascharater_bp (- (Variables|/Game/Blueprint/Charater_BP.Charater_BP_C|GetPlayerHealth _ascharater_bp) (Variables|PublicVariable|GetDamage%20per%20hit)))
    (Camera|PlayWorldCameraShake "/Game/Blueprint/HitShake_BP.HitShake_BP_C" (Transformation|GetActorLocation) 0.0 (Variables|Default|GetShakeValue))
    (Default|CallUpdateDamage _ascharater_bp true)
    (Utilities|FlowControl|Delay 0.967)
    (Default|CallUpdateDamage _ascharater_bp false)))

(event Custom|FacePlayer
  ;[1 1 1] FacePlayerEvent
  (Transformation|SetActorRotation (Math|Rotator|FindLookatRotation (Transformation|GetActorLocation) (Transformation|GetActorLocation (Game|GetPlayerCharacter 0)))))

(event Custom|CollisionEnable_LeftFist
  ;[1 1 1] Enable and Disable Fist Collision
  (Collision|SetCollisionEnabled (Variables|Default|GetLeftFist) "QueryAndPhysics"))

(event Custom|CollisionDisable_LeftFist
  ;[1 1 1] Enable and Disable Fist Collision
  (Collision|SetCollisionEnabled (Variables|Default|GetLeftFist) "NoCollision"))

(event Custom|CollisionEnable_RightFist
  ;[1 1 1] Enable and Disable Fist Collision
  (Collision|SetCollisionEnabled (Variables|Default|GetRightFist) "QueryAndPhysics"))

(event Custom|CollisionDisable_RightFist
  ;[1 1 1] Enable and Disable Fist Collision
  (Collision|SetCollisionEnabled (Variables|Default|GetRightFist) "NoCollision"))

(event EventTick
  (params (DeltaSeconds :type Float%20%28single-precision%29))
  (bind _getwspot (Variables|Default|GetGetWSpot))
  (bind _isdead (Variables|/Game/Tech/Weakspot/EnemyWeakspot_BP.EnemyWeakspot_BP_C|GetisDead _getwspot))
  ;[1 1 1] Update Alive Status
  (Utilities|IsValid _getwspot
    (:Is%20Valid
      (AI|Components|Blackboard|SetValueasBool (AI|GetBlackboard 0) (Utilities|Name|MakeLiteralName "IsDead") _isdead)
      (if _isdead
        ;[1 1 1] When Die
        (Collision|SetCollisionEnabled (Variables|Default|GetCapsuleComponent) "NoCollision")
        (CallFunction|CollisionDisableLeftFist)
        (CallFunction|CollisionDisableRightFist)
        (else
          ;[1 1 1] Update Player Distance
          (CallFunction|PlayerDistance)
          (AI|Components|Blackboard|SetValueasFloat (AI|GetBlackboard 0) (Utilities|Name|MakeLiteralName "PlayerDistance") (Variables|Default|GetPDistance))
          ;[1 1 1] Weakspot been hit
          (bind _ascharater_bp (Utilities|Casting|CastToCharater_BP (Game|GetPlayerCharacter 0)))
          (AI|Components|Blackboard|SetValueasBool (AI|GetBlackboard 0) (Utilities|Name|MakeLiteralName "beenHit") (Variables|/Game/Blueprint/Charater_BP.Charater_BP_C|GetisHitWeakspot _ascharater_bp))
          ;[1 1 1] Check Is player dead
          (bind _ascharater_bp_2 (Utilities|Casting|CastToCharater_BP (Game|GetPlayerCharacter 0)))
          (AI|Components|Blackboard|SetValueasBool (AI|GetBlackboard 0) (Utilities|Name|MakeLiteralName "IsPlayerDead") (Variables|/Game/Blueprint/Charater_BP.Charater_BP_C|GetisPlayerDead _ascharater_bp_2)))))))

(event EventBeginPlay
  (bind _returnvalue (AI|GetBlackboard 0))
  ;[1 1 1] Initialization
  (Utilities|FlowControl|Sequence
    (:then_0
      (if (Variables|PublicVariable|GetPatrol)
        (AI|Components|Blackboard|SetValueasObject (AI|GetBlackboard 0) (Utilities|Name|MakeLiteralName "PatrolPoint1") (Variables|PublicVariable|GetPoint1))
        (AI|Components|Blackboard|SetValueasObject _returnvalue (Utilities|Name|MakeLiteralName "PatrolPoint2") (Variables|PublicVariable|GetPoint2)))
      (Class|BlackboardComponent|SetValueasInt _returnvalue (Utilities|Name|MakeLiteralName "CurPoint") 1)
      (CallFunction|PlayerDistance)
      (AI|Components|Blackboard|SetValueasFloat (AI|GetBlackboard 0) (Utilities|Name|MakeLiteralName "PlayerDistance") (Variables|Default|GetPDistance))
      (AI|Components|Blackboard|SetValueasBool (AI|GetBlackboard 0) (Utilities|Name|MakeLiteralName "Attacking") false)
      (Utilities|IsValid (Variables|Default|GetGetWSpot)
        (:Is%20Valid
          (AI|Components|Blackboard|SetValueasBool (AI|GetBlackboard 0) (Utilities|Name|MakeLiteralName "IsDead") (Variables|/Game/Tech/Weakspot/EnemyWeakspot_BP.EnemyWeakspot_BP_C|GetisDead (Variables|Default|GetGetWSpot))))
        (:Is%20Not%20Valid
          _))
      (AI|Components|Blackboard|SetValueasBool (AI|GetBlackboard 0) (Utilities|Name|MakeLiteralName "CanPatrol") (Variables|PublicVariable|GetPatrol))
      (Class|BlackboardComponent|SetValueasInt (AI|GetBlackboard 0) (Utilities|Name|MakeLiteralName "RangeCheckerResult"))
      (AI|Components|Blackboard|SetValueasFloat (AI|GetBlackboard 0) (Utilities|Name|MakeLiteralName "OutRangeCD") (Variables|PublicVariable|GetOut%20Range%20Cooldown))
      (AI|Components|Blackboard|SetValueasFloat (AI|GetBlackboard 0) (Utilities|Name|MakeLiteralName "AttackRange") (Variables|PublicVariable|GetAttack%20Range))
      (AI|Components|Blackboard|SetValueasFloat (AI|GetBlackboard 0) (Utilities|Name|MakeLiteralName "SmellRange") (Variables|PublicVariable|GetSmell%20Range))
      (AI|Components|Blackboard|SetValueasFloat (AI|GetBlackboard 0) (Utilities|Name|MakeLiteralName "VibrationRange") (Variables|PublicVariable|GetVibration%20Range))
      (AI|Components|Blackboard|SetValueasFloat (AI|GetBlackboard 0) (Utilities|Name|MakeLiteralName "AttackCD") (Variables|PublicVariable|GetAttack%20Cooldown))
      (AI|Components|Blackboard|SetValueasFloat (AI|GetBlackboard 0) (Utilities|Name|MakeLiteralName "WalkSpeed") (Variables|PublicVariable|GetWalk%20Speed))
      (AI|Components|Blackboard|SetValueasFloat (AI|GetBlackboard 0) (Utilities|Name|MakeLiteralName "RunSpeed") (Variables|PublicVariable|GetRun%20Speed))
      (AI|Components|Blackboard|SetValueasBool (AI|GetBlackboard 0) (Utilities|Name|MakeLiteralName "IsPlayerDead") false)
      (AI|Components|Blackboard|SetValueasFloat (AI|GetBlackboard 0) (Utilities|Name|MakeLiteralName "SmellRange_Buff") (Variables|PublicVariable|GetSmellRange_Buff))
      (AI|Components|Blackboard|SetValueasFloat (AI|GetBlackboard 0) (Utilities|Name|MakeLiteralName "VibrationRange_Buff") (Variables|PublicVariable|GetVibrationRange_Buff))
      (AI|Components|Blackboard|SetValueasFloat (AI|GetBlackboard 0) (Utilities|Name|MakeLiteralName "RangeBuffTimer") (Variables|PublicVariable|GetRangeBuffTimer))
      (AI|Components|Blackboard|SetValueasBool (AI|GetBlackboard 0) (Utilities|Name|MakeLiteralName "HitEnemy") false)
      (AI|Components|Blackboard|SetValueasBool (AI|GetBlackboard 0) (Utilities|Name|MakeLiteralName "initialize") true)
      (Utilities|FlowControl|Delay 0.2)
      (Variables|/Game/Tech/Weakspot/EnemyWeakspot_BP.EnemyWeakspot_BP_C|SetPlantBloomHealth (Variables|Default|GetGetWSpot) (Variables|PublicVariable|GetWeakspot_Red_Health))
      (bind _output_get (Variables|/Game/Tech/Weakspot/EnemyWeakspot_BP.EnemyWeakspot_BP_C|SetPlantWiltHealth (Variables|Default|GetGetWSpot) (Variables|PublicVariable|GetWeakspot_UV_Health)))
      (Math|Float|NegateFloat _output_get
        (:%20%20
          (Variables|/Game/Tech/Weakspot/EnemyWeakspot_BP.EnemyWeakspot_BP_C|SetBatteryRate (Variables|Default|GetGetWSpot) (Variables|PublicVariable|GetBatteryDropRate))
          (Variables|/Game/Tech/Weakspot/EnemyWeakspot_BP.EnemyWeakspot_BP_C|SetSparePartRate (Variables|Default|GetGetWSpot) (Variables|PublicVariable|GetSparePartDropRate)))))
    (:then_1
      ;[1 1 1] Spawn enemy weakspot blueprint
      (bind _returnvalue_2 (Game|SpawnActorfromClass "/Game/Tech/Weakspot/EnemyWeakspot_BP.EnemyWeakspot_BP_C" (Math|Transform|MakeTransform "11.302706,-3.355629,31.370354" "-20.559906,-142.175812,6.772617" "0.200000,0.200000,0.200000") "Undefined" 0 false 4e+01))
      (bind _output_get_2 (Variables|Default|SetGetWSpot _returnvalue_2))
      (Transformation|AttachComponentToComponent (Variables|/Script/Engine.StaticMeshActor|GetStaticMeshComponent _output_get_2) (Variables|Default|GetSkeletalMesh) "Weakspot" "KeepRelative" "KeepRelative" "KeepRelative" true))))

(fn ConstructionScript)

(fn PlayerDistance
  (bind _returnvalue (Game|GetPlayerCharacter 0))
  (Utilities|IsValid _returnvalue
    (:Is%20Valid
      (Variables|Default|SetPDistance (Math|Vector|VectorLength (- (Transformation|GetActorLocation) (Transformation|GetActorLocation _returnvalue)))))))