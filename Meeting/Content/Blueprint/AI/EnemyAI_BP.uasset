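; EnemyAI_BP is an enemy AI Blueprint that reports player detection to its Blackboard through an AIPerception component.
; On each perception update, it loops over updated actors and sets SawPlayer by whether each casts to Charater_BP, so the last actor wins.
; It ignores whether sensing succeeded, so losing sight of the player still writes true.
; An unconnected alternative using Stimulus.SuccessfullySensed never runs.
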(event OnTargetPerceptionUpdated(AIPerception)
  (params (Actor :type Actor%20Object%20Reference) (Stimulus :type AI%20Stimulus%20Structure))
  ;[1 1 1] Player Detection
)

(event OnPerceptionUpdated(AIPerception)
  (params (UpdatedActors :type Array%20of%20Actor%20Object%20References))
  (for _array_element UpdatedActors
    (Utilities|Casting|CastToCharater_BP _array_element
      (:then
        (AI|Components|Blackboard|SetValueasBool (AI|GetBlackboard 0) (Utilities|Name|MakeLiteralName "SawPlayer") true))
      (:CastFailed
        (AI|Components|Blackboard|SetValueasBool (AI|GetBlackboard 0) (Utilities|Name|MakeLiteralName "SawPlayer") false)))))

(event EventBeginPlay)

(event EventTick
  (params (DeltaSeconds :type Float%20%28single-precision%29)))

(fn ConstructionScript)