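; RangeChecker is an AI behavior tree node that classifies the player's distance into attack, smell or vibration range.
; Each tick it compares the blackboard's PlayerDistance against the three range values in that order.
; The first match writes a tier number to RangeCheckerResult, and attack or smell matches also clear the Walkto flag.
; Beyond vibration range it writes nothing, so the previous result is not reset here.
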(event EventTick
  (params (OwnerActor :type Actor%20Object%20Reference) (DeltaSeconds :type Float%20%28single-precision%29))
  (bind _returnvalue (AI|GetBlackboard OwnerActor))
  (bind _returnvalue_2 (Utilities|Name|MakeLiteralName "RangeCheckerResult"))
  (bind _returnvalue_3 (AI|GetBlackboard OwnerActor))
  (bind _returnvalue_4 (Utilities|Name|MakeLiteralName "PlayerDistance"))
  (bind _returnvalue_5 (Class|BlackboardComponent|GetValueasFloat _returnvalue_3 _returnvalue_4))
  (if (<= _returnvalue_5 (Class|BlackboardComponent|GetValueasFloat _returnvalue_3 (Utilities|Name|MakeLiteralName "AttackRange")))
    (Class|BlackboardComponent|SetValueasInt _returnvalue _returnvalue_2 1)
    (Class|BTFunctionLibrary|SetBlackboardValueasBool (Variables|Default|GetWalkto) false)
    (elif (<= _returnvalue_5 (Class|BlackboardComponent|GetValueasFloat _returnvalue_3 (Utilities|Name|MakeLiteralName "SmellRange")))
      (Class|BlackboardComponent|SetValueasInt _returnvalue _returnvalue_2 2)
      (Class|BTFunctionLibrary|SetBlackboardValueasBool (Variables|Default|GetWalkto) false)
      (elif (<= _returnvalue_5 (Class|BlackboardComponent|GetValueasFloat _returnvalue_3 (Utilities|Name|MakeLiteralName "VibrationRange")))
        (Class|BlackboardComponent|SetValueasInt _returnvalue _returnvalue_2 3)))))