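; Enemy plant weakspot that visually blooms under red damage or wilts under UV damage, then drops pickups when dead.
; Tick polls externally set damage flags, stepping dissolve values on two dynamic materials, swapping between them and toggling hit particles.
; On IsDead, health against bloom/wilt thresholds (both zeroed in construction) selects final effects and drops: fruit for bloom, weighted-random battery or spare part for wilt.
; One-shot guards limit spawns, and collision is disabled.
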(event EventBeginPlay
  ;[1 1 1] Get Player Reference
  (bind _ascharater_bp (Utilities|Casting|CastToCharater_BP (Game|Player|GetPlayerPawn 0)))
  (Variables|Default|SetCharacterBP _ascharater_bp))

(event EventTick
  (params (DeltaSeconds :type Float%20%28single-precision%29))
  (bind _staticmeshcomponent (Variables|Debug|GetStaticMeshComponent))
  (Utilities|FlowControl|Sequence
    (:then_0
      (Variables|Default|SetOwnerLocation (Transformation|GetWorldLocation (Variables|Debug|GetStaticMeshComponent))))
    (:then_1
      (if (Variables|Default|GetisDead)
        (CallFunction|SetFinalEffect)
        (CallFunction|DropFruit)
        (if (not (Variables|Default|GetisRandom))
          (CallFunction|DropRate)
          (Collision|SetCollisionEnabled (Variables|Default|GetSphereCollision) "NoCollision")
          (if (== (Variables|Default|Getcounter) 0)
            (if (>= (Variables|Default|GetCurrentHealth) (Variables|Default|GetPlantBloomHealth))
              (Effects|SpawnEmitterAttached "/Game/Tech/Weakspot/NgZhiYin/Effects/Flares/P_SpotLight_DB_01.P_SpotLight_DB_01" _staticmeshcomponent "" "0, 0, 0" "64.999809,-129.999359,-179.999939" "SnapToTarget")
              (else
                (Effects|SpawnEmitterAttached "/Game/Tech/Weakspot/NgZhiYin/Effects/Flares/P_SpotLight_DB_02.P_SpotLight_DB_02" _staticmeshcomponent "" "0,0.000000, 0" "64.999809,-129.999359,-179.999939" "SnapToTarget")))
            (Variables|Default|Setcounter 1)))))
    (:then_2
      (CallFunction|SetBloomDamaged)
      (CallFunction|SetWiltDamaged))))

(fn ConstructionScript
  (bind _staticmeshcomponent (Variables|Debug|GetStaticMeshComponent))
  (Utilities|FlowControl|Sequence
    (:then_0
      (bind _returnvalue (Rendering|Material|CreateDynamicMaterialInstance _staticmeshcomponent 0 "/Game/Tech/Weakspot/Mat_Burn_Inst.Mat_Burn_Inst" :!class /Script/Engine.PrimitiveComponent))
      (Variables|Default|SetBurnMatInstance _returnvalue))
    (:then_1
      (bind _returnvalue_2 (Rendering|Material|CreateDynamicMaterialInstance _staticmeshcomponent 0 "/Game/Tech/Weakspot/Mat_Bloom_Inst.Mat_Bloom_Inst" :!class /Script/Engine.PrimitiveComponent))
      (Variables|Default|SetBloomMatInstance _returnvalue_2))
    (:then_2
      (Variables|Default|SetisDead false)
      (Variables|Default|SetisRandom false))
    (:then_3
      (bind _output_get (Variables|Default|SetPlantBloomHealth 0.0))
      (Variables|Default|SetPlantWiltHealth _output_get)
      (Variables|Default|Setcounter 0))))

(fn SetBloomDamaged
  (bind _bloommatinstance (Variables|Default|GetBloomMatInstance))
  (if (Variables|Default|GetisRedDamaged)
    (Variables|Default|SetisUV false)
    (bind _returnvalue (Rendering|Material|GetScalarParameterValue (Variables|Default|GetBurnMatInstance) "DissolveValue" :!class /Script/Engine.MaterialInstanceDynamic))
    (if (> _returnvalue 0.0)
      (Rendering|Material|SetScalarParameterValueonMaterials (Variables|Debug|GetStaticMeshComponent) "DissolveValue" (- _returnvalue 0.01))
      (else
        (if (Variables|Default|GetisRed)
          _
          (else
            (Rendering|Material|SetMaterial (Variables|Debug|GetStaticMeshComponent) 0 (Variables|Default|GetBloomMatInstance))
            (Variables|Default|SetisRed true)))
        (bind _returnvalue_2 (Rendering|Material|GetScalarParameterValue (Variables|Default|GetBloomMatInstance) "DissolveValue" :!class /Script/Engine.MaterialInstanceDynamic))
        (Rendering|Material|SetScalarParameterValueonMaterials (Variables|Debug|GetStaticMeshComponent) "DissolveValue" (+ _returnvalue_2 0.01))))
    (if (Variables|Default|GetisRedEffect)
      (Variables|Default|SetisRedDamaged false)
      (else
        (bind _returnvalue_3 (Effects|SpawnEmitterAttached "/Game/Tech/Weakspot/Leaves/P_HitEffect.P_HitEffect" (Variables|Debug|GetStaticMeshComponent) "None" "0,0.000000, 0"))
        (Variables|Default|SetParticles _returnvalue_3)
        (Variables|Default|SetisRedEffect true)
        (Variables|Default|SetisRedDamaged false)
        (bind _returnvalue_4 (Rendering|Material|GetScalarParameterValue (Variables|Default|GetBloomMatInstance) "DissolveValue" :!class /Script/Engine.MaterialInstanceDynamic))
        (if (> _returnvalue_4 1.0)
          (if (not (Variables|Default|GetisSetMaterial))
            (Rendering|Material|SetTextureParameterValue _bloommatinstance "Occlusion" "/Game/Art/Assets/Weakspot/Droid_BulbTentacles_Bloom_OcclusionRoughnessMetallic.Droid_BulbTentacles_Bloom_OcclusionRoughnessMetallic")
            (Rendering|Material|SetTextureParameterValue _bloommatinstance "Normal" "/Game/Art/Assets/Weakspot/Droid_BulbTentacles_Bloom_Normal.Droid_BulbTentacles_Bloom_Normal")
            (Rendering|Material|SetTextureParameterValue _bloommatinstance "SecondBase" "/Game/Art/Assets/Weakspot/Droid_BulbTentacles_Bloom_BaseColor.Droid_BulbTentacles_Bloom_BaseColor")
            (Rendering|Material|SetMaterial (Variables|Debug|GetStaticMeshComponent) 0 _bloommatinstance)
            (Variables|Default|SetisSetMaterial true)))))
    (elif (Variables|Default|GetisRedEffect)
      (if (Utilities|IsValid (Variables|Default|GetParticles))
        (Components|Activation|Deactivate (Variables|Default|GetParticles))
        (Variables|Default|SetisRedEffect false)))))

(fn SetWiltDamaged
  (bind _burnmatinstance (Variables|Default|GetBurnMatInstance))
  (if (Variables|Default|GetisUVDamaged)
    (Variables|Default|SetisRed false)
    (bind _returnvalue (Rendering|Material|GetScalarParameterValue (Variables|Default|GetBloomMatInstance) "DissolveValue" :!class /Script/Engine.MaterialInstanceDynamic))
    (if (> _returnvalue 0.0)
      (Rendering|Material|SetScalarParameterValueonMaterials (Variables|Debug|GetStaticMeshComponent) "DissolveValue" (- _returnvalue 0.01))
      (else
        (if (Variables|Default|GetisUV)
          _
          (else
            (Rendering|Material|SetMaterial (Variables|Debug|GetStaticMeshComponent) 0 (Variables|Default|GetBurnMatInstance))
            (Variables|Default|SetisUV true)))
        (bind _returnvalue_2 (Rendering|Material|GetScalarParameterValue (Variables|Default|GetBurnMatInstance) "DissolveValue" :!class /Script/Engine.MaterialInstanceDynamic))
        (Rendering|Material|SetScalarParameterValueonMaterials (Variables|Debug|GetStaticMeshComponent) "DissolveValue" (+ _returnvalue_2 0.01))))
    (if (Variables|Default|GetisUVEffect)
      (Variables|Default|SetisUVDamaged false)
      (else
        (bind _returnvalue_3 (Effects|SpawnEmitterAttached "/Game/Tech/Weakspot/Leaves/P_HitEffect.P_HitEffect" (Variables|Debug|GetStaticMeshComponent) "None" "0, 0, 0" "0,0.000000, 0"))
        (Variables|Default|SetParticles _returnvalue_3)
        (Variables|Default|SetisUVEffect true)
        (Variables|Default|SetisUVDamaged false)
        (bind _returnvalue_4 (Rendering|Material|GetScalarParameterValue (Variables|Default|GetBurnMatInstance) "DissolveValue" :!class /Script/Engine.MaterialInstanceDynamic))
        (if (> _returnvalue_4 1.0)
          (if (not (Variables|Default|GetisSetMaterial))
            (Rendering|Material|SetTextureParameterValue _burnmatinstance "Occlusion" "/Game/Art/Assets/Weakspot/Droid_BulbTentacles_Wilt_OcclusionRoughnessMetallic.Droid_BulbTentacles_Wilt_OcclusionRoughnessMetallic")
            (Rendering|Material|SetTextureParameterValue _burnmatinstance "Normal" "/Game/Art/Assets/Weakspot/Droid_BulbTentacles_Wilt_Normal.Droid_BulbTentacles_Wilt_Normal")
            (Rendering|Material|SetTextureParameterValue _burnmatinstance "SecondBase" "/Game/Art/Assets/Weakspot/Droid_BulbTentacles_Wilt_BaseColor.Droid_BulbTentacles_Wilt_BaseColor")
            (Rendering|Material|SetMaterial (Variables|Debug|GetStaticMeshComponent) 0 _burnmatinstance)
            (Variables|Default|SetisSetMaterial true)))))
    (elif (Variables|Default|GetisUVEffect)
      (if (Utilities|IsValid (Variables|Default|GetParticles))
        (Components|Activation|Deactivate (Variables|Default|GetParticles))
        (Variables|Default|SetisUVEffect false)))))

(fn DropBattery
  (if (<= (Variables|Default|GetCurrentHealth) (Variables|Default|GetPlantWiltHealth))
    (if (not (Variables|Default|GetIsBatterySpawned))
      (bind _output_get (Variables|Default|SetOwnerLocationOffSet ""))
      (Game|SpawnActorfromClass "/Game/Tech/InteractionSystem/Inventory/Base_Ammo/Base_HalfBattery.Base_HalfBattery_C" (Math|Conversions|ToTransform(Vector) (Math|Transform|TransformLocation _output_get (+ (Variables|Default|GetOwnerLocation) "0,50.000000, 0"))) "Undefined" 0 0)
      (Variables|Default|SetIsBatterySpawned true))
    (else
      (Variables|Default|SetIsBatterySpawned false))))

(fn DropFruit
  (if (>= (Variables|Default|GetCurrentHealth) (Variables|Default|GetPlantBloomHealth))
    (if (not (Variables|Default|GetisFruitSpawned))
      (bind _output_get (Variables|Default|SetOwnerLocationOffSet ""))
      (Game|SpawnActorfromClass "/Game/Tech/InteractionSystem/Inventory/Base_Fruit/Base_Fruit_Apple.Base_Fruit_Apple_C" (Math|Conversions|ToTransform(Vector) (Math|Transform|TransformLocation _output_get (+ (Variables|Default|GetOwnerLocation) "0.000000,50.000000,0.000000"))) "Undefined" 0 0)
      (Variables|Default|SetisFruitSpawned true))
    (else
      (Variables|Default|SetisFruitSpawned false))))

(fn DropSparePart
  (if (<= (Variables|Default|GetCurrentHealth) (Variables|Default|GetPlantWiltHealth))
    (if (not (Variables|Default|GetisSparePartSpawned))
      (bind _output_get (Variables|Default|SetOwnerLocationOffSet ""))
      (Game|SpawnActorfromClass "/Game/Tech/InteractionSystem/Inventory/Base_SparePart/Base_SparePart.Base_SparePart_C" (Math|Conversions|ToTransform(Vector) (Math|Transform|TransformLocation _output_get (+ (Variables|Default|GetOwnerLocation) "0.000000,50.000000, 0"))) "Undefined" 0 0)
      (Variables|Default|SetisSparePartSpawned true))
    (else
      (Variables|Default|SetisSparePartSpawned false))))

(fn DropRate
  (bind _output_get (Variables|Default|SetRandomValue (Math|Random|RandomIntegerinRange 1 (+ (Variables|Default|GetBatteryRate) (Variables|Default|GetSparePartRate)))))
  (if (>= (Variables|Default|GetBatteryRate) _output_get)
    (CallFunction|DropBattery)
    (Variables|Default|SetisRandom true)
    (elif (>= (+ (Variables|Default|GetBatteryRate) (Variables|Default|GetSparePartRate)) _output_get)
      (CallFunction|DropSparePart)
      (Variables|Default|SetisRandom true))))

(fn SetFinalEffect
  (Utilities|FlowControl|Sequence
    (:then_0
      (if (and (<= (Variables|Default|GetCurrentHealth) (Variables|Default|GetPlantWiltHealth)) (Math|Boolean|Equal(Boolean) (Variables|Default|GetisSpawnEmitter) false))
        (Effects|SpawnEmitterAttached "/Game/Tech/Weakspot/Leaves/P_Wilt.P_Wilt" (Variables|Debug|GetStaticMeshComponent) "None" "0.000000,0.000000, 0" "0, 0,0.000000")
        (Variables|Default|SetisSpawnEmitter true)))
    (:then_1
      (if (and (>= (Variables|Default|GetCurrentHealth) (Variables|Default|GetPlantBloomHealth)) (Math|Boolean|Equal(Boolean) (Variables|Default|GetisSpawnEmitter) false))
        (Effects|SpawnEmitterAttached "/Game/Tech/Weakspot/Blood/P_Bloom.P_Bloom" (Variables|Debug|GetStaticMeshComponent) "None" "0.000000,0.000000, 0" "0, 0,0.000000")
        (Variables|Default|SetisSpawnEmitter true)))))