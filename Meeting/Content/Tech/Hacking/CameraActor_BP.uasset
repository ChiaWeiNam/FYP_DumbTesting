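; Camera actor, filed under hacking tech, that the player steers with look input while the character's IsFPS flag is set.
; BeginPlay caches the player character and the camera's starting rotation.
; Tick adds the character's look values, pitch inverted, through four sequential limit checks, each setting rotation, so input re-applies and can override earlier clamps.
; When IsFPS is off, the camera snaps back to its starting rotation.
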(event EventTick
  (params (DeltaSeconds :type Float%20%28single-precision%29))
  (bind _cameracomponent (Variables|CameraActor|GetCameraComponent))
  (bind _cameracomponent_2 (Variables|CameraActor|GetCameraComponent))
  (bind _cameracomponent_3 (Variables|CameraActor|GetCameraComponent))
  (bind _cameracomponent_4 (Variables|CameraActor|GetCameraComponent))
  (bind _cameracomponent_5 (Variables|CameraActor|GetCameraComponent))
  (bind _cameracomponent_6 (Variables|CameraActor|GetCameraComponent))
  (bind _cameracomponent_7 (Variables|CameraActor|GetCameraComponent))
  (bind _char_ref (Variables|Default|GetChar%20Ref))
  (bind _cameracomponent_8 (Variables|CameraActor|GetCameraComponent))
  (bind _relativerotation (Variables|/Script/Engine.SceneComponent|GetRelativeRotation _cameracomponent_8))
  (bind _relativerotation_2 (Variables|/Script/Engine.SceneComponent|GetRelativeRotation _cameracomponent))
  (bind _relativerotation_3 (Variables|/Script/Engine.SceneComponent|GetRelativeRotation _cameracomponent_2))
  (bind _relativerotation_4 (Variables|/Script/Engine.SceneComponent|GetRelativeRotation _cameracomponent_3))
  (bind _relativerotation_5 (Variables|/Script/Engine.SceneComponent|GetRelativeRotation _cameracomponent_4))
  (bind _relativerotation_6 (Variables|/Script/Engine.SceneComponent|GetRelativeRotation _cameracomponent_5))
  (bind _relativerotation_7 (Variables|/Script/Engine.SceneComponent|GetRelativeRotation _cameracomponent_6))
  (bind _relativerotation_8 (Variables|/Script/Engine.SceneComponent|GetRelativeRotation _cameracomponent_7))
  (Utilities|FlowControl|Sequence
    (:then_0
      ;[1 1 1] Set Input Pitch value and Input Yaw Value
      (Variables|Default|SetLookPitchRef (Variables|/Game/Blueprint/Charater_BP.Charater_BP_C|GetLookPitchValue _char_ref))
      (Variables|Default|SetLookYawRef (Variables|/Game/Blueprint/Charater_BP.Charater_BP_C|GetLookYawValue _char_ref)))
    (:then_1
      ;[1 1 1] Control Camera Actor Rotation
      (if (Variables|/Game/Blueprint/Charater_BP.Charater_BP_C|GetIsFPS (Variables|Default|GetChar%20Ref))
        (if (>= (+ (.pitch (Variables|/Script/Engine.SceneComponent|GetRelativeRotation (Variables|CameraActor|GetCameraComponent))) (* (Variables|Default|GetLookPitchRef) -1.0)) (Variables|Default|GetMaxPitchValue))
          (Transformation|SetRelativeRotation _cameracomponent (Math|Rotator|MakeRotator (.roll _relativerotation_2) (Variables|Default|GetMaxPitchValue) (+ (.yaw _relativerotation_2) (Variables|Default|GetLookYawRef))) false false)
          (else
            (Transformation|SetRelativeRotation _cameracomponent_3 (Math|Rotator|MakeRotator (.roll _relativerotation_4) (+ (.pitch _relativerotation_4) (* (Variables|Default|GetLookPitchRef) -1.0)) (+ (.yaw _relativerotation_4) (Variables|Default|GetLookYawRef))) false false)))
        (if (<= (+ (.pitch (Variables|/Script/Engine.SceneComponent|GetRelativeRotation (Variables|CameraActor|GetCameraComponent))) (* (Variables|Default|GetLookPitchRef) -1.0)) (Variables|Default|GetMinPitchValue))
          (Transformation|SetRelativeRotation _cameracomponent_4 (Math|Rotator|MakeRotator (.roll _relativerotation_5) (Variables|Default|GetMinPitchValue) (+ (.yaw _relativerotation_5) (Variables|Default|GetLookYawRef))) false false)
          (else
            (Transformation|SetRelativeRotation _cameracomponent_2 (Math|Rotator|MakeRotator (.roll _relativerotation_3) (+ (.pitch _relativerotation_3) (* (Variables|Default|GetLookPitchRef) -1.0)) (+ (.yaw _relativerotation_3) (Variables|Default|GetLookYawRef))) false false)))
        (if (>= (+ (.yaw (Variables|/Script/Engine.SceneComponent|GetRelativeRotation (Variables|CameraActor|GetCameraComponent))) (Variables|Default|GetLookYawRef)) (Variables|Default|GetMaxYawValue))
          (Transformation|SetRelativeRotation _cameracomponent_6 (Math|Rotator|MakeRotator (.roll _relativerotation_7) (+ (.pitch _relativerotation_7) (* (Variables|Default|GetLookPitchRef) -1.0)) (Variables|Default|GetMaxYawValue)) false false)
          (else
            (Transformation|SetRelativeRotation _cameracomponent_7 (Math|Rotator|MakeRotator (.roll _relativerotation_8) (+ (.pitch _relativerotation_8) (* (Variables|Default|GetLookPitchRef) -1.0)) (+ (.yaw _relativerotation_8) (Variables|Default|GetLookYawRef))) false false)))
        (if (<= (+ (.yaw (Variables|/Script/Engine.SceneComponent|GetRelativeRotation (Variables|CameraActor|GetCameraComponent))) (Variables|Default|GetLookYawRef)) (Variables|Default|GetMinYawValue))
          (Transformation|SetRelativeRotation _cameracomponent_5 (Math|Rotator|MakeRotator (.roll _relativerotation_6) (+ (.pitch _relativerotation_6) (* (Variables|Default|GetLookPitchRef) -1.0)) (Variables|Default|GetMinYawValue)) false false)
          (else
            (Transformation|SetRelativeRotation _cameracomponent_8 (Math|Rotator|MakeRotator (.roll _relativerotation) (+ (.pitch _relativerotation) (* (Variables|Default|GetLookPitchRef) -1.0)) (+ (.yaw _relativerotation) (Variables|Default|GetLookYawRef))) false false)))
        (else
          (Transformation|SetRelativeRotation (Variables|CameraActor|GetCameraComponent) (Math|Rotator|MakeRotator (Variables|Default|GetOriginalRollValue) (Variables|Default|GetOriginalPitchValue) (Variables|Default|GetOriginalYawValue)) false false))))))

(event EventBeginPlay
  (bind _cameracomponent (Variables|CameraActor|GetCameraComponent))
  (bind _relativerotation (Variables|/Script/Engine.SceneComponent|GetRelativeRotation _cameracomponent))
  (Utilities|FlowControl|Sequence
    (:then_0
      ;[1 1 1] Cast to Character Ref
      (bind _ascharater_bp (Utilities|Casting|CastToCharater_BP (Game|Player|GetPlayerPawn 0)))
      (Variables|Default|SetChar%20Ref _ascharater_bp))
    (:then_1
      ;[1 1 1] Set Original Rotation Value
      (Transformation|SetRelativeRotation _cameracomponent (Math|Rotator|MakeRotator (.roll _relativerotation) (.pitch _relativerotation) (.yaw _relativerotation)) false false)
      (Variables|Default|SetOriginalRollValue (.roll _relativerotation))
      (Variables|Default|SetOriginalPitchValue (.pitch _relativerotation))
      (Variables|Default|SetOriginalYawValue (.yaw _relativerotation)))))

(fn ConstructionScript)