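; PC_Solo4 is an interactable that switches the player to a fixed camera view with a PinDoor_UI pin-door widget.
; A box overlap notifies the player character's entry and exit through the radius handlers.
; When IsFPS is false, OnInteract sets it, hides and teleports the character to the camera, blends the view there and shows the widget with the cursor.
; Interacting again only clears the flag, without restoring view or input.
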(event OnComponentBeginOverlap(Box)
  (params (OverlappedComponent :type Primitive%20Component%20Object%20Reference) (OtherActor :type Actor%20Object%20Reference) (OtherComp :type Primitive%20Component%20Object%20Reference) (OtherBodyIndex :type Integer) (bFromSweep :type Boolean) (SweepResult :type Hit%20Result%20Structure%20%28by%20ref%29))
  (bind _ascharater_bp (Utilities|Casting|CastToCharater_BP OtherActor))
  (CallFunction|OnPlayerEnterRadius self _ascharater_bp))

(event OnComponentEndOverlap(Box)
  (params (OverlappedComponent :type Primitive%20Component%20Object%20Reference) (OtherActor :type Actor%20Object%20Reference) (OtherComp :type Primitive%20Component%20Object%20Reference) (OtherBodyIndex :type Integer))
  (bind _ascharater_bp (Utilities|Casting|CastToCharater_BP OtherActor))
  (CallFunction|OnPlayerLeaveRadius self _ascharater_bp))

(event EventOnInteract
  (params (Character :type Charater%20BP%20Object%20Reference))
  (bind _returnvalue (Game|GetPlayerController 0))
  (bind _charref (Variables|Default|GetCharRef))
  (if (Variables|/Game/Blueprint/Charater_BP.Charater_BP_C|GetIsFPS _charref)
    (Variables|/Game/Blueprint/Charater_BP.Charater_BP_C|SetIsFPS _charref false)
    (else
      (Variables|/Game/Blueprint/Charater_BP.Charater_BP_C|SetIsFPS _charref true)
      (Rendering|SetActorHiddenInGame _charref true)
      (Game|Player|SetViewTargetwithBlend (Game|GetPlayerController 0) (Variables|Default|GetCameraRef) 0.5 "VTBlend_Linear" 0.0 true)
      (bind _returnvalue_2 (UserInterface|CreateWidget "/Game/Tech/PinDoor/PinDoor_UI.PinDoor_UI_C"))
      (bind _output_get (Variables|Default|SetPinDoorRef _returnvalue_2))
      (UserInterface|Viewport|AddtoViewport _output_get 0)
      (Input|SetInputModeGameandUI _returnvalue 0 "DoNotLock" true)
      (Variables|/Script/Engine.PlayerController|SetbShowMouseCursor _returnvalue true)
      (Transformation|SetActorLocation (Variables|Default|GetCharRef) (Transformation|GetActorLocation (Variables|Default|GetCameraRef)) false false))))

(event EventBeginPlay
  (bind _ascharater_bp (Utilities|Casting|CastToCharater_BP (Game|Player|GetPlayerPawn 0)))
  (Variables|Default|SetCharRef _ascharater_bp))

(fn ConstructionScript)