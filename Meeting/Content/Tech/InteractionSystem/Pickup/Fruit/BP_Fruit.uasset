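; BP_Fruit is an interactable pickup that disappears when used and flags the player character as having picked up health.
; On BeginPlay it caches the player character and writes its name into the interaction widget.
; Box overlaps with the character fire enter and leave radius events that show or hide that widget.
; OnInteract destroys the actor and sets IsPickupHealth on the cached character, while the construction script enlarges the mesh.
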(event OnComponentBeginOverlap(Box)
  (params (OverlappedComponent :type Primitive%20Component%20Object%20Reference) (OtherActor :type Actor%20Object%20Reference) (OtherComp :type Primitive%20Component%20Object%20Reference) (OtherBodyIndex :type Integer) (bFromSweep :type Boolean) (SweepResult :type Hit%20Result%20Structure%20%28by%20ref%29))
  ;[1 1 1] Start Colliding with other actor
  (bind _ascharater_bp (Utilities|Casting|CastToCharater_BP OtherActor))
  (CallFunction|OnPlayerEnterRadius self _ascharater_bp))

(event OnComponentEndOverlap(Box)
  (params (OverlappedComponent :type Primitive%20Component%20Object%20Reference) (OtherActor :type Actor%20Object%20Reference) (OtherComp :type Primitive%20Component%20Object%20Reference) (OtherBodyIndex :type Integer))
  ;[1 1 1] Start Colliding with other actor
  (bind _ascharater_bp (Utilities|Casting|CastToCharater_BP OtherActor))
  (CallFunction|OnPlayerLeaveRadius self _ascharater_bp))

(event EventOnPlayerEnterRadius
  (params (Character :type Charater%20BP%20Object%20Reference))
  ;[1 1 1] OnEnter/Leave Player Radius
  (Rendering|SetVisibility (Variables|Default|GetWidget) true false))

(event EventOnPlayerLeaveRadius
  (params (Character :type Charater%20BP%20Object%20Reference))
  ;[1 1 1] OnEnter/Leave Player Radius
  (Rendering|SetVisibility (Variables|Default|GetWidget) false false))

(event EventBeginPlay
  (Utilities|FlowControl|Sequence
    (:then_0
      ;[1 1 1] Casting To Character_BP
      (bind _ascharater_bp (Utilities|Casting|CastToCharater_BP (Game|Player|GetPlayerPawn 0)))
      (Variables|Default|SetCharacterBP _ascharater_bp))
    (:then_1
      ;[1 1 1] Event BeginPlay
      (bind _asinteraction_widget (Utilities|Casting|CastToInteractionWidget (UserInterface|GetUserWidgetObject (Variables|Default|GetWidget))))
      (Rendering|Components|TextRender|SetText (Variables|/Game/Tech/InteractionSystem/InteractionWidget.InteractionWidget_C|GetName _asinteraction_widget) (Variables|Default|GetName)))))

(event EventOnInteract
  (params (Character :type Charater%20BP%20Object%20Reference))
  ;[1 1 1] Interaction Event
  (Actor|DestroyActor)
  (Variables|/Game/Blueprint/Charater_BP.Charater_BP_C|SetbIsPickupHealth (Variables|Default|GetCharacterBP) true))

(fn ConstructionScript
  (Transformation|SetWorldScale3D (Variables|Default|GetStaticMesh) "3.000000,3.000000,3.000000"))