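; Interactable door Blueprint that opens via a Matinee, optionally gated by a hacking terminal when locked.
; On interact, if unlocked or the terminal's CanOpen is set, it plays the Matinee and animates twelve GUI skeletal mesh layers, then hides them and resets their poses.
; When a Charater_BP leaves the trigger box, it reverses the Matinee after a short delay, then shows the GUI layers again.
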(event OnComponentEndOverlap(Box)
  (params (OverlappedComponent :type Primitive%20Component%20Object%20Reference) (OtherActor :type Actor%20Object%20Reference) (OtherComp :type Primitive%20Component%20Object%20Reference) (OtherBodyIndex :type Integer))
  ;[1 1 1] Colliding Set Up
  (bind _ascharater_bp (Utilities|Casting|CastToCharater_BP OtherActor))
  (CallFunction|OnPlayerLeaveRadius self _ascharater_bp))

(event EventOnPlayerLeaveRadius
  (params (Character :type Charater%20BP%20Object%20Reference) (BasePickup :type Base%20Pickup%20Object%20Reference))
  ;[1 1 1] Player Leave Radius
  (Utilities|FlowControl|Delay 0.5)
  (Utilities|String|Reverse (Variables|Default|GetMatineeRef))
  (Utilities|FlowControl|Delay 2.0)
  (Rendering|SetVisibility (Variables|/Script/Engine.SkeletalMeshActor|GetSkeletalMeshComponent (Variables|Default|GetGUI_Layer1)) true false)
  (Rendering|SetVisibility (Variables|/Script/Engine.SkeletalMeshActor|GetSkeletalMeshComponent (Variables|Default|GetGUI_Layer2)) true false)
  (Rendering|SetVisibility (Variables|/Script/Engine.SkeletalMeshActor|GetSkeletalMeshComponent (Variables|Default|GetGUI_Layer3)) true false)
  (Rendering|SetVisibility (Variables|/Script/Engine.SkeletalMeshActor|GetSkeletalMeshComponent (Variables|Default|GetGUI_Layer4)) true false)
  (Rendering|SetVisibility (Variables|/Script/Engine.SkeletalMeshActor|GetSkeletalMeshComponent (Variables|Default|GetGUI_Layer5)) true false)
  (Rendering|SetVisibility (Variables|/Script/Engine.SkeletalMeshActor|GetSkeletalMeshComponent (Variables|Default|GetGUI_Layer6)) true false)
  (Rendering|SetVisibility (Variables|/Script/Engine.SkeletalMeshActor|GetSkeletalMeshComponent (Variables|Default|GetGUI_Layer7)) true false)
  (Rendering|SetVisibility (Variables|/Script/Engine.SkeletalMeshActor|GetSkeletalMeshComponent (Variables|Default|GetGUI_Layer8)) true false)
  (Rendering|SetVisibility (Variables|/Script/Engine.SkeletalMeshActor|GetSkeletalMeshComponent (Variables|Default|GetGUI_Layer9)) true false)
  (Rendering|SetVisibility (Variables|/Script/Engine.SkeletalMeshActor|GetSkeletalMeshComponent (Variables|Default|GetGUI_Layer10)) true false)
  (Rendering|SetVisibility (Variables|/Script/Engine.SkeletalMeshActor|GetSkeletalMeshComponent (Variables|Default|GetGUI_Layer11)) true false)
  (Rendering|SetVisibility (Variables|/Script/Engine.SkeletalMeshActor|GetSkeletalMeshComponent (Variables|Default|GetGUI_Layer12)) true false))

(event EventOnInteract
  (params (Character :type Charater%20BP%20Object%20Reference))
  ;[1 1 1] Interact
  (if (Variables|Default|GetisLockedDoor?)
    (if (Variables|/Game/Tech/InteractionSystem/Hacking_Terminal_UI_Blueprint.Hacking_Terminal_UI_Blueprint_C|GetCanOpen? (Variables|Default|GetHacking%20Terminal%20UI%20Ref))
      (Audio|Components|Audio|Play (Variables|Default|GetMatineeRef) :!label _label)
      (Components|Animation|PlayAnimation (Variables|/Script/Engine.SkeletalMeshActor|GetSkeletalMeshComponent (Variables|Default|GetGUI_Layer1)) "/Game/Art/DoorUI/ANIMATION_Plane001_Anim.ANIMATION_Plane001_Anim" false)
      (Components|Animation|PlayAnimation (Variables|/Script/Engine.SkeletalMeshActor|GetSkeletalMeshComponent (Variables|Default|GetGUI_Layer2)) "/Game/Art/DoorUI/ANIMATION_Object003_Anim.ANIMATION_Object003_Anim" false)
      (Components|Animation|PlayAnimation (Variables|/Script/Engine.SkeletalMeshActor|GetSkeletalMeshComponent (Variables|Default|GetGUI_Layer3)) "/Game/Art/DoorUI/ANIMATION_Object004_Anim.ANIMATION_Object004_Anim" false)
      (Components|Animation|PlayAnimation (Variables|/Script/Engine.SkeletalMeshActor|GetSkeletalMeshComponent (Variables|Default|GetGUI_Layer4)) "/Game/Art/DoorUI/ANIMATION_Object005_Anim.ANIMATION_Object005_Anim" false)
      (Components|Animation|PlayAnimation (Variables|/Script/Engine.SkeletalMeshActor|GetSkeletalMeshComponent (Variables|Default|GetGUI_Layer5)) "/Game/Art/DoorUI/ANIMATION_Object006_Anim.ANIMATION_Object006_Anim" false)
      (Components|Animation|PlayAnimation (Variables|/Script/Engine.SkeletalMeshActor|GetSkeletalMeshComponent (Variables|Default|GetGUI_Layer6)) "/Game/Art/DoorUI/ANIMATION_Object007_Anim.ANIMATION_Object007_Anim" false)
      (Components|Animation|PlayAnimation (Variables|/Script/Engine.SkeletalMeshActor|GetSkeletalMeshComponent (Variables|Default|GetGUI_Layer7)) "/Game/Art/DoorUI/ANIMATION_Plane001_Anim.ANIMATION_Plane001_Anim" false)
      (Components|Animation|PlayAnimation (Variables|/Script/Engine.SkeletalMeshActor|GetSkeletalMeshComponent (Variables|Default|GetGUI_Layer8)) "/Game/Art/DoorUI/ANIMATION_Object003_Anim.ANIMATION_Object003_Anim" false)
      (Components|Animation|PlayAnimation (Variables|/Script/Engine.SkeletalMeshActor|GetSkeletalMeshComponent (Variables|Default|GetGUI_Layer9)) "/Game/Art/DoorUI/ANIMATION_Object004_Anim.ANIMATION_Object004_Anim" false)
      (Components|Animation|PlayAnimation (Variables|/Script/Engine.SkeletalMeshActor|GetSkeletalMeshComponent (Variables|Default|GetGUI_Layer10)) "/Game/Art/DoorUI/ANIMATION_Object005_Anim.ANIMATION_Object005_Anim" false)
      (Components|Animation|PlayAnimation (Variables|/Script/Engine.SkeletalMeshActor|GetSkeletalMeshComponent (Variables|Default|GetGUI_Layer11)) "/Game/Art/DoorUI/ANIMATION_Object006_Anim.ANIMATION_Object006_Anim" false)
      (Components|Animation|PlayAnimation (Variables|/Script/Engine.SkeletalMeshActor|GetSkeletalMeshComponent (Variables|Default|GetGUI_Layer12)) "/Game/Art/DoorUI/ANIMATION_Object007_Anim.ANIMATION_Object007_Anim" false)
      (Utilities|FlowControl|Delay 1.333)
      (Rendering|SetVisibility (Variables|/Script/Engine.SkeletalMeshActor|GetSkeletalMeshComponent (Variables|Default|GetGUI_Layer1)) false false)
      (Rendering|SetVisibility (Variables|/Script/Engine.SkeletalMeshActor|GetSkeletalMeshComponent (Variables|Default|GetGUI_Layer2)) false false)
      (Rendering|SetVisibility (Variables|/Script/Engine.SkeletalMeshActor|GetSkeletalMeshComponent (Variables|Default|GetGUI_Layer3)) false false)
      (Rendering|SetVisibility (Variables|/Script/Engine.SkeletalMeshActor|GetSkeletalMeshComponent (Variables|Default|GetGUI_Layer4)) false false)
      (Rendering|SetVisibility (Variables|/Script/Engine.SkeletalMeshActor|GetSkeletalMeshComponent (Variables|Default|GetGUI_Layer5)) false false)
      (Rendering|SetVisibility (Variables|/Script/Engine.SkeletalMeshActor|GetSkeletalMeshComponent (Variables|Default|GetGUI_Layer6)) false false)
      (Rendering|SetVisibility (Variables|/Script/Engine.SkeletalMeshActor|GetSkeletalMeshComponent (Variables|Default|GetGUI_Layer7)) false false)
      (Rendering|SetVisibility (Variables|/Script/Engine.SkeletalMeshActor|GetSkeletalMeshComponent (Variables|Default|GetGUI_Layer8)) false false)
      (Rendering|SetVisibility (Variables|/Script/Engine.SkeletalMeshActor|GetSkeletalMeshComponent (Variables|Default|GetGUI_Layer9)) false false)
      (Rendering|SetVisibility (Variables|/Script/Engine.SkeletalMeshActor|GetSkeletalMeshComponent (Variables|Default|GetGUI_Layer10)) false false)
      (Rendering|SetVisibility (Variables|/Script/Engine.SkeletalMeshActor|GetSkeletalMeshComponent (Variables|Default|GetGUI_Layer11)) false false)
      (Rendering|SetVisibility (Variables|/Script/Engine.SkeletalMeshActor|GetSkeletalMeshComponent (Variables|Default|GetGUI_Layer12)) false false)
      (Components|Animation|SetAnimation (Variables|/Script/Engine.SkeletalMeshActor|GetSkeletalMeshComponent (Variables|Default|GetGUI_Layer1)) "/Game/Art/DoorUI/Start_Pose/Plane001_Pose.Plane001_Pose")
      (Components|Animation|SetAnimation (Variables|/Script/Engine.SkeletalMeshActor|GetSkeletalMeshComponent (Variables|Default|GetGUI_Layer2)) "/Game/Art/DoorUI/Start_Pose/Object003_Pose.Object003_Pose")
      (Components|Animation|SetAnimation (Variables|/Script/Engine.SkeletalMeshActor|GetSkeletalMeshComponent (Variables|Default|GetGUI_Layer3)) "/Game/Art/DoorUI/Start_Pose/Object004_Pose.Object004_Pose")
      (Components|Animation|SetAnimation (Variables|/Script/Engine.SkeletalMeshActor|GetSkeletalMeshComponent (Variables|Default|GetGUI_Layer4)) "/Game/Art/DoorUI/Start_Pose/Object005_Pose.Object005_Pose")
      (Components|Animation|SetAnimation (Variables|/Script/Engine.SkeletalMeshActor|GetSkeletalMeshComponent (Variables|Default|GetGUI_Layer5)) "/Game/Art/DoorUI/Start_Pose/Object006_Pose.Object006_Pose")
      (Components|Animation|SetAnimation (Variables|/Script/Engine.SkeletalMeshActor|GetSkeletalMeshComponent (Variables|Default|GetGUI_Layer6)) "/Game/Art/DoorUI/Start_Pose/Object007_Pose.Object007_Pose")
      (Components|Animation|SetAnimation (Variables|/Script/Engine.SkeletalMeshActor|GetSkeletalMeshComponent (Variables|Default|GetGUI_Layer7)) "/Game/Art/DoorUI/Start_Pose/Plane001_Pose.Plane001_Pose")
      (Components|Animation|SetAnimation (Variables|/Script/Engine.SkeletalMeshActor|GetSkeletalMeshComponent (Variables|Default|GetGUI_Layer8)) "/Game/Art/DoorUI/Start_Pose/Object003_Pose.Object003_Pose")
      (Components|Animation|SetAnimation (Variables|/Script/Engine.SkeletalMeshActor|GetSkeletalMeshComponent (Variables|Default|GetGUI_Layer9)) "/Game/Art/DoorUI/Start_Pose/Object004_Pose.Object004_Pose")
      (Components|Animation|SetAnimation (Variables|/Script/Engine.SkeletalMeshActor|GetSkeletalMeshComponent (Variables|Default|GetGUI_Layer10)) "/Game/Art/DoorUI/Start_Pose/Object005_Pose.Object005_Pose")
      (Components|Animation|SetAnimation (Variables|/Script/Engine.SkeletalMeshActor|GetSkeletalMeshComponent (Variables|Default|GetGUI_Layer11)) "/Game/Art/DoorUI/Start_Pose/Object006_Pose.Object006_Pose")
      (Components|Animation|SetAnimation (Variables|/Script/Engine.SkeletalMeshActor|GetSkeletalMeshComponent (Variables|Default|GetGUI_Layer12)) "/Game/Art/DoorUI/Start_Pose/Object007_Pose.Object007_Pose"))
    (else
      (goto _label))))

(fn ConstructionScript)