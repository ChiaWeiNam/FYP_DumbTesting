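; SteamPanel_BP is a hackable terminal controlling a timed steam hazard for enemies.
; Interacting toggles a blended camera zoom, hiding and moving the player to the camera and showing the MiniGame_UI widget, unless the hack is complete.
; Tick polls IsActivateSteam to enable steam particles and a trigger box, then shuts them off after a minute and clears CompleteHack.
; The trigger box sets InSteam on overlapping enemies.
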(event OnActorBeginOverlap(TriggerBox1)
  (params (OverlappedActor :type Actor%20Object%20Reference) (OtherActor :type Actor%20Object%20Reference))
  ;[1 1 1] Inform enemy in steam
  (bind _asenemy_chracter_bp (Utilities|Casting|CastToEnemyChracter_BP OtherActor))
  (Variables|/Game/Blueprint/AI/EnemyChracter_BP.EnemyChracter_BP_C|SetInSteam _asenemy_chracter_bp true))

(event OnActorEndOverlap(TriggerBox1)
  (params (OverlappedActor :type Actor%20Object%20Reference) (OtherActor :type Actor%20Object%20Reference))
  ;[1 1 1] Inform enemy in steam
  (bind _asenemy_chracter_bp (Utilities|Casting|CastToEnemyChracter_BP OtherActor))
  (Variables|/Game/Blueprint/AI/EnemyChracter_BP.EnemyChracter_BP_C|SetInSteam _asenemy_chracter_bp false))

(event EventTick
  (params (DeltaSeconds :type Float%20%28single-precision%29))
  (bind _steamevent (Variables|Default|GetSteamEvent))
  (bind _triggerbox1 (Variables|Default|GetTriggerBox1))
  (if (Variables|Default|GetisActivateSteam?)
    (for _array_element _steamevent
      (Components|Activation|SetActive (Variables|/Script/Engine.Emitter|GetParticleSystemComponent _array_element) true false)
      (Collision|SetActorEnableCollision _triggerbox1 true))
    (Variables|Default|SetisActivateSteam? false)
    (Variables|Default|SetisTimerStart true)
    (elif (Variables|Default|GetisTimerStart)
      (Utilities|FlowControl|Delay 6e+01)
      (for _array_element_2 _steamevent
        (Components|Activation|SetActive (Variables|/Script/Engine.Emitter|GetParticleSystemComponent _array_element_2) false false)
        (Collision|SetActorEnableCollision _triggerbox1 false))
      (Variables|Default|SetisTimerStart false)
      (Variables|Default|SetCompleteHack? false))))

(event EventOnInteract
  (params (Character :type Charater%20BP%20Object%20Reference))
  (bind _returnvalue (Game|GetPlayerController 0))
  (bind _returnvalue_2 (Game|GetPlayerController 0))
  (bind _charref (Variables|Default|GetCharRef))
  (bind _charref_2 (Variables|Default|GetCharRef))
  (if (not (Variables|Default|GetCompleteHack?))
    ;[1 1 1] Hacking Terminal Zoom In Control
    (if (Variables|/Game/Blueprint/Charater_BP.Charater_BP_C|GetIsFPS _charref_2)
      (Variables|/Game/Blueprint/Charater_BP.Charater_BP_C|SetIsFPS _charref_2 false)
      (Rendering|SetActorHiddenInGame _charref false)
      (Game|Player|SetViewTargetwithBlend (Game|GetPlayerController 0) _charref 0.5 "VTBlend_Linear" 0.0 false)
      (Widget|RemovefromParent (Variables|Default|GetMiniGameRef))
      (Variables|Default|SetMiniGameIsValid false)
      (Input|SetInputModeGameOnly _returnvalue_2)
      (Variables|/Script/Engine.PlayerController|SetbShowMouseCursor _returnvalue_2 false)
      (else
        (Variables|/Game/Blueprint/Charater_BP.Charater_BP_C|SetIsFPS _charref_2 true)
        (Rendering|SetActorHiddenInGame _charref_2 true)
        (Game|Player|SetViewTargetwithBlend (Game|GetPlayerController 0) (Variables|Default|GetCameraRef) 0.5 "VTBlend_Linear" 0.0 true)
        (bind _returnvalue_3 (UserInterface|CreateWidget "/Game/Tech/MiniGame/MiniGame_UI.MiniGame_UI_C"))
        (bind _output_get (Variables|Default|SetMiniGameRef _returnvalue_3))
        (UserInterface|Viewport|AddtoViewport _output_get 0)
        (Variables|Default|SetMiniGameIsValid true)
        (Input|SetInputModeGameandUI _returnvalue 0 "DoNotLock" true)
        (Variables|/Script/Engine.PlayerController|SetbShowMouseCursor _returnvalue true)
        (Transformation|SetActorLocation (Variables|Default|GetCharRef) (Transformation|GetActorLocation (Variables|Default|GetCameraRef)) false false)))))

(event EventBeginPlay
  ;[1 1 1] Character Ref
  (bind _ascharater_bp (Utilities|Casting|CastToCharater_BP (Game|Player|GetPlayerPawn 0)))
  (Variables|Default|SetCharRef _ascharater_bp)
  ;[1 1 1] Initialize Trigger Box
  (Collision|SetActorEnableCollision (Variables|Default|GetTriggerBox1) false))

(fn ConstructionScript)